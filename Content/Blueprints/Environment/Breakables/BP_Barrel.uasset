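; Breakable barrel that drops a random pickup when the actor is destroyed.
; The Destroyed event rolls a random integer to spawn a gem, coin or croissant with equal odds, slightly below the barrel's origin.
; The Blueprint holds no damage or break logic of its own, and its construction script only calls the parent.
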(event `self.ReceiveDestroyed`
  (bind _returnvalue (`KismetMathLibrary.MakeTransform` (- (`self.K2_GetActorLocation`) (0.0 0.0 50.0))))
  (switch `int` (`KismetMathLibrary.RandomIntegerInRange` 0 2)
    (:`0`
      (`|SpawnActorFromClass` "/Game/Blueprints/Pickups/BP_Gem.BP_Gem_C" _returnvalue "Undefined" "OverrideRootScale" null null))
    (:`1`
      (`|SpawnActorFromClass` "/Game/Blueprints/Pickups/BP_Coin.BP_Coin_C" _returnvalue "Undefined" "OverrideRootScale" null null))
    (:`2`
      (`|SpawnActorFromClass` "/Game/Blueprints/Pickups/BP_Croissant.BP_Croissant_C" _returnvalue "Undefined" "OverrideRootScale" null null))))

(fn `UserConstructionScript`
  (`parent.UserConstructionScript`))