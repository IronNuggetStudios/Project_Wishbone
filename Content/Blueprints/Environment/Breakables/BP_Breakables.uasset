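; BP_Breakables is a breakable environment actor that reacts to overlapping BP_ProjectileOLD projectiles and is destroyed once its hit count reaches MaxHits.
; Below that limit, a timeline animates the static mesh's scale, incrementing CurrentHit and clearing the Hit gate on every update rather than once per hit.
; At the limit, a second timeline lerps the mesh from StartScale to EndScale, and a delay started from its update leads to DestroyActor.
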(event `self.ReceiveActorBeginOverlap`
  (params (OtherActor :type "Actor Object Reference"))
  (if (not (`self.Hit`))
    (cast `/Game/Blueprints/Projectiles/BP_ProjectileOLD` OtherActor)
    (set `self.Hit` true)
    (if (>= (`self.CurrentHit`) (`self.MaxHits`))
      (bind (_direction _scalealpha) (`Timeline|Scale` :!via `PlayFromStart`)
        (:`Update`
          (`SceneComponent.SetRelativeScale3D` (`self.StaticMesh`) (`KismetMathLibrary.VLerp` (`self.Start Scale`) (`self.End Scale`) _scalealpha))
          (`KismetSystemLibrary.Delay` 0.5)
          (`self.K2_DestroyActor`)))
      (else
        (bind (_direction_2 _scale) (`Timeline|Timeline_0` :!via `PlayFromStart`)
          (:`Update`
            (`SceneComponent.SetRelativeScale3D` (`self.StaticMesh`) _scale)
            (`/Engine/EditorBlueprintResources/StandardMacros.IncrementInt` (`self.CurrentHit`)
              (:`  `
                (set `self.Hit` false)))))))))

(fn `UserConstructionScript`)