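; BP_Column is a breakable environment column that degrades when a BP_ProjectileMaster actor overlaps it.
; Below MaxHits, an overlap plays a scale timeline whose update also increments CurrentHit.
; At two thresholds it destroys groups of mesh pieces and spawns BP_Debris at a random point inside its Box.
; Once CurrentHit reaches MaxHits, the next overlap lerps the actor's scale and destroys it after a short delay.
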(event `self.ReceiveActorBeginOverlap`
  (params (OtherActor :type "Actor Object Reference"))
  (bind _box (`self.Box`))
  (cast `/Game/Blueprints/Projectiles/BP_ProjectileMaster` OtherActor)
  (if (>= (`self.CurrentHit`) (`self.MaxHits`))
    (bind (_direction _scalealpha) (`Timeline|Scale` :!via `PlayFromStart`)
      (:`Update`
        (`self.SetActorScale3D` (`KismetMathLibrary.VLerp` (`self.Start Scale`) (`self.End Scale`) _scalealpha))
        (`KismetSystemLibrary.Delay` 0.5)
        (`self.K2_DestroyActor`)))
    (else
      (bind (_direction_2 _scale) (`Timeline|Timeline_0` :!via `PlayFromStart`)
        (:`Update`
          (`self.SetActorScale3D` _scale)
          (`/Engine/EditorBlueprintResources/StandardMacros.IncrementInt` (`self.CurrentHit`)
            (:`  `
              (switch `int` (`self.CurrentHit`)
                (:`2`
                  (`ActorComponent.K2_DestroyComponent` (`self.StaticMesh12`))
                  (`ActorComponent.K2_DestroyComponent` (`self.StaticMesh11`))
                  (`ActorComponent.K2_DestroyComponent` (`self.StaticMesh13`))
                  (`ActorComponent.K2_DestroyComponent` (`self.StaticMesh14`))
                  (`ActorComponent.K2_DestroyComponent` (`self.StaticMesh15`)))
                (:`5`
                  (`ActorComponent.K2_DestroyComponent` (`self.StaticMesh4`))
                  (`ActorComponent.K2_DestroyComponent` (`self.StaticMesh7`))
                  (`ActorComponent.K2_DestroyComponent` (`self.StaticMesh5`))
                  (`ActorComponent.K2_DestroyComponent` (`self.StaticMesh8`))
                  (`ActorComponent.K2_DestroyComponent` (`self.StaticMesh10`))
                  (`ActorComponent.K2_DestroyComponent` (`self.StaticMesh9`))))
              (`|SpawnActorFromClass` "/Game/Blueprints/Projectiles/BP_Debris.BP_Debris_C" (`KismetMathLibrary.Conv_VectorToTransform` (`KismetMathLibrary.RandomPointInBoundingBox` (`SceneComponent.K2_GetComponentLocation` _box) (`BoxComponent.GetScaledBoxExtent` _box))) "Undefined" "OverrideRootScale" null null))))))))

(fn `UserConstructionScript`)