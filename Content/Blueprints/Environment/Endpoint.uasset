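; Endpoint is a room exit trigger that ends the current room when the player reaches it.
; On BeginPlay it caches references to the game mode and player controller.
; When the player overlaps its box and the game mode reports the room cleared, it saves the game, fades the camera and audio out, then after a short delay tells the game mode the room is complete.
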(event `self.ReceiveBeginPlay`
  (bind _asbp_game_mode (cast `/Game/Blueprints/BP_GameMode` (`GameplayStatics.GetGameMode`)))
  (set `self.GameModeRef` _asbp_game_mode)
  (bind _asbp_player_controller (cast `/Game/Blueprints/BP_PlayerController` (`GameplayStatics.GetPlayerController` 0)))
  (set `self.PlayerControllerRef` _asbp_player_controller))

(event `self.Box.OnComponentBeginOverlap`
  (params (OverlappedComponent :type "PrimitiveComponent Object Reference") (OtherActor :type "Actor Object Reference") (OtherComp :type "PrimitiveComponent Object Reference") (OtherBodyIndex :type Integer) (bFromSweep :type Boolean) (SweepResult :type "HitResult Structure (by ref)"))
  (cast `/Game/Blueprints/BP_Player` OtherActor)
  (if (`/Game/Blueprints/BP_GameMode.RoomCleared` (`self.GameModeRef`))
    (`/Game/Blueprints/BP_PlayerController.SaveGame` (`self.PlayerControllerRef`))
    (`PlayerCameraManager.StartCameraFade` :`self` (`GameplayStatics.GetPlayerCameraManager` 0) :`ToAlpha` 1.0 :`Duration` 0.25 :`bShouldFadeAudio` true :`bHoldWhenFinished` true)
    (`KismetSystemLibrary.Delay` 0.25)
    (`/Game/Blueprints/BP_GameMode.RoomComplete` (`self.GameModeRef`))))

(fn `UserConstructionScript`)