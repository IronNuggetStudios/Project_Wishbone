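; Spikes1 is a floor spike trap that sinks its mesh on BeginPlay and springs it up when the player enters its trigger box.
; The box overlap arms a Spiked flag, waits briefly, raises the spikes with an eased MoveComponentTo, then disarms and lowers them after another delay.
; While armed, any actor that begins overlapping the spike mesh takes fixed damage.
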(event `self.ReceiveBeginPlay`
  (bind _staticmesh1 (`self.StaticMesh1`))
  (`KismetSystemLibrary.MoveComponentTo` _staticmesh1 (+ (`SceneComponent.RelativeLocation` _staticmesh1) (0.0 0.0 -100.0)) (struct) true true))

(event `self.Box.OnComponentBeginOverlap`
  (params (OverlappedComponent :type "PrimitiveComponent Object Reference") (OtherActor :type "Actor Object Reference") (OtherComp :type "PrimitiveComponent Object Reference") (OtherBodyIndex :type Integer) (bFromSweep :type Boolean) (SweepResult :type "HitResult Structure (by ref)"))
  (bind _staticmesh1 (`self.StaticMesh1`))
  (bind _staticmesh1_2 (`self.StaticMesh1`))
  (cast `/Game/Blueprints/BP_Player` OtherActor)
  (set `self.Spiked` true)
  (`KismetSystemLibrary.Delay` 0.5)
  (`KismetSystemLibrary.MoveComponentTo` _staticmesh1_2 (+ (`SceneComponent.RelativeLocation` _staticmesh1_2) (0.0 0.0 100.0)) (struct) true true)
  (`KismetSystemLibrary.Delay` 0.5)
  (set `self.Spiked` false)
  (`KismetSystemLibrary.MoveComponentTo` _staticmesh1 (+ (`SceneComponent.RelativeLocation` _staticmesh1) (0.0 0.0 -100.0)) (struct) true true))

(event `self.StaticMesh1.OnComponentBeginOverlap`
  (params (OverlappedComponent :type "PrimitiveComponent Object Reference") (OtherActor :type "Actor Object Reference") (OtherComp :type "PrimitiveComponent Object Reference") (OtherBodyIndex :type Integer) (bFromSweep :type Boolean) (SweepResult :type "HitResult Structure (by ref)"))
  (if (`self.Spiked`)
    (`GameplayStatics.ApplyDamage` OtherActor 20.0)))

(fn `UserConstructionScript`)