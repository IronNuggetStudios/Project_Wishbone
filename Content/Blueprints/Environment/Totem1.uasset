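; Totem1 is a clickable environment totem that spawns melee slime enemies.
; A looping timer set on BeginPlay calls Spawn, which creates a BP_SlimeAI pawn running BT_MeleeAI at a random point inside the Box component's extent around the totem.
; Each spawn's rotation comes from the totem-to-player direction.
; Clicking the static mesh destroys the totem.
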(event `self.ReceiveBeginPlay`
  (`KismetSystemLibrary.K2_SetTimer` null "Spawn" 0.0 true))

(event `self.StaticMesh.OnClicked`
  (params (TouchedComponent :type "PrimitiveComponent Object Reference") (ButtonPressed :type "Key Structure"))
  (`self.K2_DestroyActor`))

(fn `Spawn`
  (bind _returnvalue (`self.K2_GetActorLocation`))
  (`AIBlueprintHelperLibrary.SpawnAIFromClass` "/Game/Blueprints/AI/BP_SlimeAI.BP_SlimeAI_C" "/Game/Blueprints/AI/BaseAI/BT_MeleeAI.BT_MeleeAI" (`KismetMathLibrary.RandomPointInBoundingBox` _returnvalue (`BoxComponent.GetScaledBoxExtent` (`self.Box`))) (`KismetMathLibrary.FindLookAtRotation` _returnvalue (`self.K2_GetActorLocation` (`GameplayStatics.GetPlayerCharacter` 0)))))

(fn `UserConstructionScript`)