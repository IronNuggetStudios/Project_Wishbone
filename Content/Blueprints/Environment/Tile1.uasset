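; Tile1 is an environment Blueprint that builds a flat grid of block meshes with randomly varied orientations.
; The Construction Script loops over Width and Length, spacing blocks by Xoffset and Yoffset and picking one of seven preset rotations for each.
; AddBlockToInstance adds each block to a single Instanced Static Mesh component.
; The random picks are unseeded, so the layout can change whenever construction reruns, and no runtime event logic is active.
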(fn `AddBlockToInstance`
  (params (Location :type "Vector Structure") (Rotation :type "Rotator Structure"))
  (`InstancedStaticMeshComponent.AddInstance` (`self.InstancedStaticMesh`) (`KismetMathLibrary.MakeTransform` Location Rotation)))

(fn `UserConstructionScript`
  (for _index (range (+ (`self.Width`) 1))
    (for _index_2 (range (+ (`self.Length`) 1))
      (switch `int` (`KismetMathLibrary.RandomIntegerInRange` 0 6)
        (:`0`
          (bind _returnvalue (`KismetMathLibrary.MakeVector` (`KismetMathLibrary.Conv_IntToDouble` (* _index_2 (`self.Xoffset`))) (`KismetMathLibrary.Conv_IntToDouble` (* _index (`self.Yoffset`)))))
          (`self.AddBlockToInstance` _returnvalue (struct)))
        (:`1`
          (`self.AddBlockToInstance` _returnvalue (struct :`Roll` 90.0)))
        (:`2`
          (`self.AddBlockToInstance` _returnvalue (struct :`Pitch` 90.0)))
        (:`3`
          (`self.AddBlockToInstance` _returnvalue (struct :`Pitch` 90.0 :`Yaw` 90.0)))
        (:`4`
          (`self.AddBlockToInstance` _returnvalue (struct :`Yaw` 90.0)))
        (:`5`
          (`self.AddBlockToInstance` _returnvalue (struct :`Yaw` 180.0)))
        (:`6`
          (`self.AddBlockToInstance` _returnvalue (struct :`Yaw` 270.0)))))))