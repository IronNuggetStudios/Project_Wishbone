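; EndDoor1 is a barred door that raises when the player enters its trigger box and lowers when they leave.
; Box overlap events filtered to BP_Player use MoveComponentTo with easing to shift Bars1 up or down.
; Each move targets an offset from the bars' current relative location, so overlapping again mid-motion can drift the rest position.
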(event `self.Box.OnComponentBeginOverlap`
  (params (OverlappedComponent :type "PrimitiveComponent Object Reference") (OtherActor :type "Actor Object Reference") (OtherComp :type "PrimitiveComponent Object Reference") (OtherBodyIndex :type Integer) (bFromSweep :type Boolean) (SweepResult :type "HitResult Structure (by ref)"))
  (bind _bars1 (`self.Bars1`))
  (cast `/Game/Blueprints/BP_Player` OtherActor)
  (`KismetSystemLibrary.MoveComponentTo` _bars1 (+ (`SceneComponent.RelativeLocation` _bars1) (0.0 0.0 300.0)) (struct) true true))

(event `self.Box.OnComponentEndOverlap`
  (params (OverlappedComponent :type "PrimitiveComponent Object Reference") (OtherActor :type "Actor Object Reference") (OtherComp :type "PrimitiveComponent Object Reference") (OtherBodyIndex :type Integer))
  (bind _bars1 (`self.Bars1`))
  (cast `/Game/Blueprints/BP_Player` OtherActor)
  (`KismetSystemLibrary.MoveComponentTo` _bars1 (+ (`SceneComponent.RelativeLocation` _bars1) (0.0 0.0 -300.0)) (struct) true true))

(fn `UserConstructionScript`)