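; Wave spawner that fills its Box volume with randomly chosen AI enemies whenever BP_GameMode reports a wave has ended.
; BeginPlay runs the first check; Tick uses Delays to periodically call UpdateWave on the game mode, then repeat it.
; Each new wave increments WaveNumber, clears WaveEnded and spawns MaxEnemies at random points in the box.
; Picks are melee slimes or ranged honeypot ants; SpawnSlimeDaddy currently spawns the same class as SpawnSlime.
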(event `self.ReceiveBeginPlay`
  (bind _asbp_game_mode (cast `/Game/Blueprints/BP_GameMode` (`GameplayStatics.GetGameMode`)))
  (if (`/Game/Blueprints/BP_GameMode.WaveEnded` _asbp_game_mode) :!label _label
    (bind _result (`/Engine/EditorBlueprintResources/StandardMacros.IncrementInt` (`/Game/Blueprints/BP_GameMode.WaveNumber` _asbp_game_mode))
      (:`  `
        (`KismetSystemLibrary.PrintString` (`KismetStringLibrary.Concat_StrStr` "Wave " (`KismetStringLibrary.Conv_IntToString` _result)))
        (set `/Game/Blueprints/BP_GameMode.WaveEnded` false _asbp_game_mode)
        (for _index (range (`/Game/Blueprints/BP_GameMode.MaxEnemies` _asbp_game_mode))
          (switch `int` (`KismetMathLibrary.RandomIntegerInRange` 0 2)
            (:`0`
              (`self.SpawnSlime`))
            (:`1`
              (`self.SpawnSlimeDaddy`))
            (:`2`
              (`self.SpawnHoneypotAnt`))))
        (`KismetSystemLibrary.PrintString` (`KismetStringLibrary.Concat_StrStr` (`KismetStringLibrary.Conv_IntToString` _index) " Enemies"))))))

(event `self.ReceiveTick`
  (params (DeltaSeconds :type "Float (single-precision)"))
  (`KismetSystemLibrary.Delay` 3.0)
  (`/Game/Blueprints/BP_GameMode.UpdateWave` (stale `self.ReceiveBeginPlay` _asbp_game_mode))
  (`KismetSystemLibrary.Delay` 1.0)
  (goto _label))

(fn `SpawnHoneypotAnt`
  (bind _box (`self.Box`))
  (`AIBlueprintHelperLibrary.SpawnAIFromClass` "/Game/Blueprints/AI/BP_HoneypotAnt.BP_HoneypotAnt_C" "/Game/Blueprints/AI/BaseAI/BT_RangedAI.BT_RangedAI" (`KismetMathLibrary.RandomPointInBoundingBox` (`SceneComponent.K2_GetComponentLocation` _box) (`BoxComponent.BoxExtent` _box))))

(fn `SpawnSlime`
  (bind _box (`self.Box`))
  (`AIBlueprintHelperLibrary.SpawnAIFromClass` "/Game/Blueprints/AI/BP_SlimeAI.BP_SlimeAI_C" "/Game/Blueprints/AI/BaseAI/BT_MeleeAI.BT_MeleeAI" (`KismetMathLibrary.RandomPointInBoundingBox` (`SceneComponent.K2_GetComponentLocation` _box) (`BoxComponent.BoxExtent` _box))))

(fn `SpawnSlimeDaddy`
  (bind _box (`self.Box`))
  (`AIBlueprintHelperLibrary.SpawnAIFromClass` "/Game/Blueprints/AI/BP_SlimeAI.BP_SlimeAI_C" "/Game/Blueprints/AI/BaseAI/BT_MeleeAI.BT_MeleeAI" (`KismetMathLibrary.RandomPointInBoundingBox` (`SceneComponent.K2_GetComponentLocation` _box) (`BoxComponent.BoxExtent` _box))))

(fn `UserConstructionScript`)