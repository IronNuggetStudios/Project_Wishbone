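; BP_Croissant is a single-use health pickup that heals the player on overlap.
; It takes a random yaw at BeginPlay, then on first player overlap calls HealPlayer on BP_PlayerController with its Health value.
; A timeline lerps the mesh scale from StartScale to EndScale, and a Delay chained to its Update pin destroys the actor half a second after the animation begins.
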(event `self.ReceiveBeginPlay`
  (`self.K2_SetActorRotation` (`KismetMathLibrary.MakeRotator` 0.0 0.0 (`KismetMathLibrary.RandomFloatInRange` 0.0 360.0))))

(event `self.ReceiveActorBeginOverlap`
  (params (OtherActor :type "Actor Object Reference"))
  (if (not (`self.Used`))
    (bind _asbp_player (cast `/Game/Blueprints/BP_Player` OtherActor))
    (bind _asbp_player_controller (cast `/Game/Blueprints/BP_PlayerController` (`Pawn.GetController` _asbp_player)))
    (`/Game/Blueprints/BP_PlayerController.HealPlayer` _asbp_player_controller (`self.Health`))
    (set `self.Used` true)
    (bind (_direction _scalealpha) (`Timeline|Scale` :`NewTime` 0.0)
      (:`Update`
        (`SceneComponent.SetRelativeScale3D` (`self.StaticMesh`) (`KismetMathLibrary.VLerp` (`self.Start Scale`) (`self.End Scale`) _scalealpha))
        (`KismetSystemLibrary.Delay` 0.5)
        (`self.K2_DestroyActor`)))))

(fn `UserConstructionScript`)