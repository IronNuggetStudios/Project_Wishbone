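; BP_ProjectileOLD is a projectile that deals radial damage on overlap or stop, with an optional nova burst.
; BeginPlay applies Scale and destroys it after one second if still unresolved.
; A Complete flag guards the timeout, stop and overlap paths against repeat handling.
; On overlap only, Nova yaws the Cube in even steps, spawning a BP_NovaOLD from the Box transform at each, before a briefly delayed destroy.
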(event `self.ReceiveBeginPlay`
  (`self.SetActorScale3D` (`self.Scale`))
  (`KismetSystemLibrary.Delay` 1.0)
  (if (not (`self.Complete`))
    (set `self.Complete` true)
    (`self.K2_DestroyActor`)))

(event `self.ProjectileMovement.OnProjectileStop`
  (params (ImpactResult :type "HitResult Structure (by ref)"))
  (if (not (`self.Complete`))
    (`GameplayStatics.ApplyRadialDamage` :`BaseDamage` (`self.Damage`) :`Origin` (`SceneComponent.K2_GetComponentLocation` (`self.Cube`)) :`DamageRadius` 200.0 :`DamageCauser` null :`InstigatedByController` null)
    (set `self.Complete` true)
    (`self.K2_DestroyActor`)))

(event `self.Cube.OnComponentBeginOverlap`
  (params (OverlappedComponent :type "PrimitiveComponent Object Reference") (OtherActor :type "Actor Object Reference") (OtherComp :type "PrimitiveComponent Object Reference") (OtherBodyIndex :type Integer) (bFromSweep :type Boolean) (SweepResult :type "HitResult Structure (by ref)"))
  (if (not (`self.Complete`))
    (`GameplayStatics.ApplyRadialDamage` :`BaseDamage` (`self.Damage`) :`Origin` (`SceneComponent.K2_GetComponentLocation` (`self.Cube`)) :`DamageRadius` 200.0 :`DamageCauser` null :`InstigatedByController` null)
    (if (`self.IsNova`)
      (`self.Nova` (`self.ProjectileCount`)))
    (set `self.Complete` true)
    (`KismetSystemLibrary.Delay` 0.1)
    (`self.K2_DestroyActor`)))

(fn `Nova`
  (params (ProjectileCount :type Integer))
  (if (`self.IsNova`)
    (for _ (range ProjectileCount)
      (bind _output_get (set `self.Rotation` (+ (`self.Rotation`) (`KismetMathLibrary.Conv_IntToDouble` (/ 360 ProjectileCount)))))
      (`SceneComponent.K2_SetWorldRotation` (`self.Cube`) (`KismetMathLibrary.MakeRotator` 0.0 0.0 _output_get) false false)
      (`|SpawnActorFromClass` "/Game/Blueprints/Projectiles/BP_NovaOLD.BP_NovaOLD_C" (`SceneComponent.K2_GetComponentToWorld` (`self.Box`)) "Undefined" "OverrideRootScale" null null))))

(fn `UserConstructionScript`)