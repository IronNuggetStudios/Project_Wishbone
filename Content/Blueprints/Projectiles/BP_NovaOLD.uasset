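; BP_NovaOLD is a projectile that explodes for radial damage when it comes to a stop.
; The ProjectileMovement stop event applies Damage in a fixed radius around the Cube component, then destroys the actor.
; A Complete flag guards against repeat detonation.
; An unconnected copy of this logic, gated on a cast to BP_BaseAI, never runs.
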(event `self.ProjectileMovement.OnProjectileStop`
  (params (ImpactResult :type "HitResult Structure (by ref)"))
  (if (not (`self.Complete`))
    (`GameplayStatics.ApplyRadialDamage` :`BaseDamage` (`self.Damage`) :`Origin` (`SceneComponent.K2_GetComponentLocation` (`self.Cube`)) :`DamageRadius` 200.0 :`DamageCauser` null :`InstigatedByController` null)
    (set `self.Complete` true)
    (`self.K2_DestroyActor`)))

(fn `UserConstructionScript`)