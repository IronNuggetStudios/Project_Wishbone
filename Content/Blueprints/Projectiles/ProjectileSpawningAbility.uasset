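; ProjectileSpawningAbility is a reusable ability that fires a BP_Projectile toward a target location.
; A setup event stores the spawn point and projectile speed.
; The firing event spawns the projectile at the spawn point's world transform, then overwrites its Cube's physics linear velocity with the unit direction to the target scaled by that speed.
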(event `Setup Projectile Ability`
  (params (Spawnpoint :type "PrimitiveComponent Object Reference") (ProjectileSpeed :type "Float (double-precision)"))
  (set `self.Spawnpoint` Spawnpoint)
  (set `self.ProjectileSpeed` ProjectileSpeed))

(event `Spawn Projectile At Target`
  (params (TargetLocation :type "Vector Structure"))
  (bind _returnvalue_location (`KismetMathLibrary.BreakTransform` (`SceneComponent.K2_GetComponentToWorld` (`self.Spawnpoint`))))
  (set `self.TargetLocation` TargetLocation)
  (bind _returnvalue (`|SpawnActorFromClass` "/Game/Blueprints/Projectiles/BP_Projectile.BP_Projectile_C" (`SceneComponent.K2_GetComponentToWorld` (`self.Spawnpoint`)) "Undefined" "OverrideRootScale" null null))
  (`PrimitiveComponent.SetAllPhysicsLinearVelocity` (`/Game/Blueprints/Projectiles/BP_Projectile.Cube` _returnvalue) (* (`KismetMathLibrary.GetDirectionUnitVector` _returnvalue_location (`self.TargetLocation`)) (`self.ProjectileSpeed`)) false))