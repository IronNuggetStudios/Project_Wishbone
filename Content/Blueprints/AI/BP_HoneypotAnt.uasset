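; BP_HoneypotAnt is an ant AI Blueprint that releases a slime enemy through its PlayFX event.
; BeginPlay runs the parent logic, then initializes health, barrier and damage.
; PlayFX spawns a BP_SlimeAI running BT_MeleeAI at a random point within the Box component's extent around the ant.
; The slime's rotation is computed to look from the ant toward the player.
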(event `self.ReceiveBeginPlay`
  (`parent.ReceiveBeginPlay`)
  (`self.Initialize Hitpoints` 25.0 25.0 25.0 25.0 0.0 3.0))

(event `self.Play FX`
  (bind _returnvalue (`self.K2_GetActorLocation`))
  (`AIBlueprintHelperLibrary.SpawnAIFromClass` "/Game/Blueprints/AI/BP_SlimeAI.BP_SlimeAI_C" "/Game/Blueprints/AI/BaseAI/BT_MeleeAI.BT_MeleeAI" (`KismetMathLibrary.RandomPointInBoundingBox` _returnvalue (`BoxComponent.GetScaledBoxExtent` (`self.Box`))) (`KismetMathLibrary.FindLookAtRotation` _returnvalue (`self.K2_GetActorLocation` (`GameplayStatics.GetPlayerCharacter` 0)))))

(fn `UserConstructionScript`
  (`parent.UserConstructionScript`))