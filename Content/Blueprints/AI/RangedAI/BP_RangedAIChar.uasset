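; BP_RangedAIChar is a ranged AI character that attacks a given enemy with hitscan damage.
; AttackEnemy sets Attacking, calls the empty PlayFX event, then line-traces on the Camera channel from itself to the enemy.
; If the trace hits that enemy, it applies Damage and clears Attacking after a two-second delay.
; A missed or blocked trace leaves Attacking set.
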(event `Attack Enemy`
  (params (EnemyToAttack :type "Actor Object Reference"))
  (set `self.Attacking` true)
  (`self.Play FX`)
  (bind (_outhit _returnvalue) (`KismetSystemLibrary.LineTraceSingle` (`self.K2_GetActorLocation`) (`self.K2_GetActorLocation` EnemyToAttack) "TraceTypeQuery2" true))
  (if _returnvalue
    (bind (_bblockinghit _binitialoverlap _time _distance _location _impactpoint _normal _impactnormal _physmat _hitactor) (`GameplayStatics.BreakHitResult` _outhit))
    (if (== _hitactor EnemyToAttack)
      (`GameplayStatics.ApplyDamage` _hitactor (`self.Damage`) (`self.GetController`) self "/Script/Engine.DamageType")
      (`KismetSystemLibrary.Delay` 2.0)
      (set `self.Attacking` false))))

(event `Play FX`)

(fn `UserConstructionScript`)