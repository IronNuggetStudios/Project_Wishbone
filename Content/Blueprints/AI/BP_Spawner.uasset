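; BP_Spawner is an AI spawner that populates the level with a batch of slime enemies when play begins.
; BeginPlay calls Spawn, which loops and randomly picks BP_SlimeDaddyAI or BP_SlimeAI on each pass, both running the BT_MeleeAI behavior tree.
; Only BP_SlimeAI gets a random location inside the Box extents around the actor; the SlimeDaddy spawn sets no location.
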(event `self.ReceiveBeginPlay`
  (`self.Spawn`))

(fn `Spawn`
  (for _ (range 11)
    (switch `int` (`KismetMathLibrary.RandomIntegerInRange` 0 1)
      (:`0`
        (`AIBlueprintHelperLibrary.SpawnAIFromClass` "/Game/Blueprints/AI/BP_SlimeDaddyAI.BP_SlimeDaddyAI_C" "/Game/Blueprints/AI/BaseAI/BT_MeleeAI.BT_MeleeAI"))
      (:`1`
        (`AIBlueprintHelperLibrary.SpawnAIFromClass` "/Game/Blueprints/AI/BP_SlimeAI.BP_SlimeAI_C" "/Game/Blueprints/AI/BaseAI/BT_MeleeAI.BT_MeleeAI" (`KismetMathLibrary.RandomPointInBoundingBox` (`self.K2_GetActorLocation`) (`BoxComponent.GetScaledBoxExtent` (`self.Box`))))))))

(fn `UserConstructionScript`)