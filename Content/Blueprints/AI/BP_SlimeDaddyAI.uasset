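; BP_SlimeDaddyAI is a slime enemy that splits into smaller slimes when destroyed.
; On BeginPlay it runs the parent logic, then initializes its health and damage.
; While Attacking, a Box overlap with BP_Player applies damage to the Enemy reference rather than directly to the overlapped actor.
; Its Destroyed event spawns a random number of BP_SlimeAI pawns running the BT_MeleeAI behavior tree.
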(event `self.ReceiveBeginPlay`
  (`parent.ReceiveBeginPlay`)
  (`self.Initialize Hitpoints` 100.0 100.0 0.0 0.0 0.0 3.0))

(event `self.ReceiveDestroyed`
  (for _ (range (+ (`KismetMathLibrary.RandomIntegerInRange` 0 3) 1))
    (`AIBlueprintHelperLibrary.SpawnAIFromClass` "/Game/Blueprints/AI/BP_SlimeAI.BP_SlimeAI_C" "/Game/Blueprints/AI/MeleeAI/BT_MeleeAI.BT_MeleeAI")))

(event `self.Box.OnComponentBeginOverlap`
  (params (OverlappedComponent :type "PrimitiveComponent Object Reference") (OtherActor :type "Actor Object Reference") (OtherComp :type "PrimitiveComponent Object Reference") (OtherBodyIndex :type Integer) (bFromSweep :type Boolean) (SweepResult :type "HitResult Structure (by ref)"))
  (if (`self.Attacking`)
    (cast `/Game/Blueprints/BP_Player` OtherActor)
    (`GameplayStatics.ApplyDamage` (`self.Enemy`) (`self.Damage`) (`self.GetController`) self "/Script/Engine.DamageType")))

(fn `UserConstructionScript`
  (`parent.UserConstructionScript`))