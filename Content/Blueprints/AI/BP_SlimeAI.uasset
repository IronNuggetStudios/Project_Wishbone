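; BP_SlimeAI is the slime AI character, which sets its health and damage stats and deals contact damage to the player.
; BeginPlay runs the parent logic, then initializes its hitpoints and damage.
; When its Box overlaps a BP_Player while Attacking is set, it applies damage to the stored Enemy reference rather than directly to the overlapping actor.
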(event `self.ReceiveBeginPlay`
  (`parent.ReceiveBeginPlay`)
  (`self.Initialize Hitpoints` 25.0 25.0 0.0 0.0 0.0 3.0))

(event `self.Box.OnComponentBeginOverlap`
  (params (OverlappedComponent :type "PrimitiveComponent Object Reference") (OtherActor :type "Actor Object Reference") (OtherComp :type "PrimitiveComponent Object Reference") (OtherBodyIndex :type Integer) (bFromSweep :type Boolean) (SweepResult :type "HitResult Structure (by ref)"))
  (if (`self.Attacking`)
    (cast `/Game/Blueprints/BP_Player` OtherActor)
    (`GameplayStatics.ApplyDamage` (`self.Enemy`) (`self.Damage`) (`self.GetController`) self "/Script/Engine.DamageType")))

(fn `UserConstructionScript`
  (`parent.UserConstructionScript`))