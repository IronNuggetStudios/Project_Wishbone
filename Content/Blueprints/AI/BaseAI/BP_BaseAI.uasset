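; Base AI enemy character with health, barrier, melee and ranged attacks, and a widget health bar linked on BeginPlay.
; Damage drains the barrier first and spills into health, updating the bar and material overlay; the actor is destroyed only by hits taken without barrier.
; Melee only animates the overlay via timeline.
; Ranged attack calls an empty PlayFX hook, then line-traces to player 0 and applies damage on hit.
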(event `self.ReceiveBeginPlay`
  (bind _asbp_aihealth_bar (cast `/Game/Blueprints/UI/BP_AIHealthBar` (`WidgetComponent.GetUserWidgetObject` (`self.AIBar`))))
  (set `/Game/Blueprints/UI/BP_AIHealthBar.AI` self _asbp_aihealth_bar))

(event `/Game/Blueprints/AI/BaseAI/CombatInterface.MeleeAttack`
  (set `self.Attacking` true)
  (bind (_direction _scalaroverlay) (`Timeline|Fade to white` :!via `PlayFromStart`)
    (:`Update`
      (`MeshComponent.SetScalarParameterValueOnMaterials` (`self.Mesh`) "Overlay" _scalaroverlay))
    (:`Finished`
      (`KismetSystemLibrary.Delay` 1.0)
      (set `self.Attacking` false))))

(event `Play FX`)

(event `/Game/Blueprints/AI/BaseAI/CombatInterface.RangedAttack`
  (bind _returnvalue (`GameplayStatics.GetPlayerCharacter` 0))
  (set `self.Attacking` true)
  (`self.Play FX`)
  (bind (_outhit _returnvalue_2) (`KismetSystemLibrary.LineTraceSingle` (`self.K2_GetActorLocation`) (`self.K2_GetActorLocation` _returnvalue) "TraceTypeQuery2" true))
  (if _returnvalue_2
    (bind (_bblockinghit _binitialoverlap _time _distance _location _impactpoint _normal _impactnormal _physmat _hitactor) (`GameplayStatics.BreakHitResult` _outhit))
    (if (== _hitactor _returnvalue)
      (`GameplayStatics.ApplyDamage` _hitactor (`self.Damage`) (`self.GetController`) self "/Script/Engine.DamageType"))
    (`KismetSystemLibrary.Delay` 1.0)
    (set `self.Attacking` false)))

(event `self.ReceiveAnyDamage`
  (params (Damage :type "Float (single-precision)") (DamageType :type "DamageType Object Reference") (InstigatedBy :type "Controller Object Reference") (DamageCauser :type "Actor Object Reference"))
  (`self.TakeDamage` Damage))

(fn `Initialize Hitpoints`
  (params (CurrentHealth :type "Float (double-precision)") (MaxHealth :type "Float (double-precision)") (CurrentBarrier :type "Float (double-precision)") (MaxBarrier :type "Float (double-precision)") (BarrierRegen :type "Float (double-precision)") (Damage :type "Float (double-precision)"))
  (set `self.CurrentHealth` CurrentHealth)
  (set `self.MaxHealth` MaxHealth)
  (set `self.CurrentBarrier` CurrentBarrier)
  (set `self.MaxBarrier` MaxBarrier)
  (set `self.BarrierRegen` BarrierRegen)
  (set `self.Damage` Damage)
  (`self.UpdateHealth` (`self.CurrentHealth`))
  (`self.UpdateBarrier` (`self.CurrentBarrier`)))

(fn `TakeDamage`
  (params (Damage :type "Float (double-precision)"))
  (`MeshComponent.SetScalarParameterValueOnMaterials` (`self.Mesh`) "Overlay" 0.0)
  (if (== (`self.CurrentBarrier`) 0.0)
    (bind _output_get (set `self.CurrentHealth` (- (`self.CurrentHealth`) Damage)))
    (if (<= _output_get 0.0)
      (`self.K2_DestroyActor`)
      (else
        (`self.UpdateHealth` _output_get)
        (`MeshComponent.SetScalarParameterValueOnMaterials` (`self.Mesh`) "Overlay" 0.5 :!label _label)))
    (else
      (bind _output_get_2 (set `self.CurrentBarrier` (- (`self.CurrentBarrier`) Damage)))
      (if (<= _output_get_2 0.0)
        (bind _output_get_3 (set `self.CurrentHealth` (+ (`self.CurrentHealth`) _output_get_2)))
        (`self.UpdateHealth` _output_get_3)
        (bind _output_get_4 (set `self.CurrentBarrier` 0.0))
        (`self.UpdateBarrier` _output_get_4)
        (goto _label)
        (else
          (`self.UpdateBarrier` _output_get_2)
          (goto _label))))))

(fn `UserConstructionScript`)