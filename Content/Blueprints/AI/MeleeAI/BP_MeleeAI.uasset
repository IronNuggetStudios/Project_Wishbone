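; BP_MeleeAI is a melee AI unit with health, barrier, barrier regen and damage stats, plus a widget-based status bar.
; On BeginPlay it passes itself to its BP_MeleeAIBar widget.
; InitializeHitpoints stores the supplied stats and triggers the health and barrier update calls.
; MeleeAttack records the target enemy and holds an Attacking flag for a short delay, without applying damage in this graph.
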(event `self.ReceiveBeginPlay`
  (bind _asbp_melee_aibar (cast `/Game/Blueprints/UI/BP_MeleeAIBar` (`WidgetComponent.GetUserWidgetObject` (`self.MeleeAIBar`))))
  (set `/Game/Blueprints/UI/BP_MeleeAIBar.MeleeAI` self _asbp_melee_aibar))

(event `/Game/Blueprints/AI/MeleeAI/CombatInterface.MeleeAttack`
  (params (EnemyToAttack :type "Actor Object Reference"))
  (set `self.Enemy` EnemyToAttack)
  (set `self.Attacking` true)
  (`KismetSystemLibrary.Delay` 1.0)
  (set `self.Attacking` false))

(fn `Initialize Hitpoints`
  (params (CurrentHealth :type "Float (double-precision)") (MaxHealth :type "Float (double-precision)") (CurrentBarrier :type "Float (double-precision)") (MaxBarrier :type "Float (double-precision)") (BarrierRegen :type "Float (double-precision)") (Damage :type "Float (double-precision)"))
  (set `self.CurrentHealth` CurrentHealth)
  (set `self.MaxHealth` MaxHealth)
  (set `self.CurrentBarrier` CurrentBarrier)
  (set `self.MaxBarrier` MaxBarrier)
  (set `self.BarrierRegen` BarrierRegen)
  (set `self.Damage` Damage)
  (`self.UpdateHealth` (`self.CurrentHealth`))
  (`self.UpdateBarrier` (`self.CurrentBarrier`)))

(fn `UserConstructionScript`)